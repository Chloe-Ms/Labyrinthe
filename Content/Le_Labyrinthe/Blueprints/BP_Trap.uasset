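; BP_Trap is a labyrinth trap that moves two wall cubes toward each other's starting positions when an actor overlaps it.
; The overlap prints a warning, caches both cubes' world locations and plays a timeline whose Alpha lerps each cube along that path without sweep.
; An IsMoving flag blocks retriggering until the timeline finishes.
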(event Custom|eventMoveCube
  (params (Cube :type Static%20Mesh%20Component%20Object%20Reference) (Start :type Vector) (End :type Vector) (alpha :type Float%20%28double-precision%29))
  (Transformation|SetWorldLocation Cube (Math|Vector|Lerp(Vector) Start End alpha) false false))

(event EventBeginPlay)

(event Collision|EventActorBeginOverlap
  (params (OtherActor :type Actor%20Object%20Reference))
  (if (not (Variables|Default|GetIsMoving))
    (Variables|Default|SetIsMoving true)
    (Development|PrintString "WATCH OUT")
    (Variables|Default|SetInitialPositionCube (Transformation|GetWorldLocation (Variables|Default|GetCube)))
    (Variables|Default|SetInitialPositionCube1 (Transformation|GetWorldLocation (Variables|Default|GetCube1)))
    ;[1 1 1] Active the trap ( the two walls move)
    (bind _alpha (Timeline|TimelineLerpTrap Play)
      (:Update
        (CallFunction|EventMoveCube (Variables|Default|GetCube) (Variables|Default|GetInitialPositionCube) (Variables|Default|GetInitialPositionCube1) _alpha)
        (CallFunction|EventMoveCube (Variables|Default|GetCube1) (Variables|Default|GetInitialPositionCube1) (Variables|Default|GetInitialPositionCube) _alpha))
      (:Finished
        (Variables|Default|SetIsMoving false)))))

(fn ConstructionScript)