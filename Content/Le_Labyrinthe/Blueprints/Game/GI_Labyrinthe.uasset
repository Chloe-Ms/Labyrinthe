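; Game instance for the labyrinth game that tracks two puzzle conditions, a lit torch and a turned-on switch, to open a secret passage.
; The torch and switch events each set their flag and run a shared condition check.
; When both flags are true, the check prints a message and instantly shifts every actor tagged "PassageSecret" upward, with no guard against repeated moves.
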(event Custom|eventTurnSwitchOn
  (Variables|Default|SetIsSwitchOn true)
  (CallFunction|EventCheckConditionstoOpenDoor))

(event Custom|eventLightTorch
  (Variables|Default|SetIsTorchLit true)
  (CallFunction|EventCheckConditionstoOpenDoor))

(event Custom|eventCheckConditionsToOpenDoor
  (if (Variables|Default|GetIsTorchLit)
    (if (Variables|Default|GetIsSwitchOn)
      (Development|PrintString "The door is open")
      (bind _outactors (Actor|GetAllActorswithTag "PassageSecret"))
      (for _array_element _outactors
        (Transformation|SetActorLocation _array_element (+ (Transformation|GetActorLocation _array_element) "0.000000,0.000000,100.000000") false false)))))